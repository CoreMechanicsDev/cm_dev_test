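; BP_NPC_Jeanne is the Jeanne NPC, with helpers for cycling patrol points and turning smoothly.
; Tick runs an RInterpTo loop toward TargetRotationResult while ShouldRotate is set, flagging RotationComplete within tolerance.
; GetNextLocation and GetNextRotation read actor locations from ACPathNode's PatrolPath and advance separate wrapping indices.
; GetNextRotation reads at LocationIndex but advances RotationIndex, and stores a location as NextRotation.
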(event `self.ReceiveBeginPlay`)

(event `self.ReceiveTick`
  (params (DeltaSeconds :type "Float (single-precision)"))
  (if (`self.bShouldRotate`)
    (`self.DoRotationLoop`)))

(event `DoRotationLoop`
  (set `self.bRotationComplete` false)
  ; Rotation Loop
  (`self.K2_SetActorRotation` (`KismetMathLibrary.RInterpTo` (`self.K2_GetActorRotation`) (`self.TargetRotationResult`) (`GameplayStatics.GetWorldDeltaSeconds`) 3.0))
  (if (== (`self.K2_GetActorRotation`) (`self.TargetRotationResult`) :`ErrorTolerance` 2.0)
    (set `self.bShouldRotate` false)
    (set `self.bRotationComplete` true)
    (`KismetSystemLibrary.PrintString` "ROTATION COMPLETE")))

(fn `GetNextLocation`
  ; Get next patrol point from array
  (set `self.NextLocation` (`self.K2_GetActorLocation` (`|GetArrayItem` (`/Game/AI/AC_PatrolPath.PatrolPath` (`self.AC_PathNode`)) (`self.LocationIndex`))))
  ; Check if we're at last path point
  (if (>= (`self.LocationIndex`) (- (`KismetArrayLibrary.Array_Length` (`/Game/AI/AC_PatrolPath.PatrolPath` (`self.AC_PathNode`))) 1))
    ; If yes, reset index, otherwise bump
    (set `self.LocationIndex` 0)
    (else
      (`/Engine/EditorBlueprintResources/StandardMacros.IncrementInt` (`self.LocationIndex`)))))

(fn `GetNextRotation`
  ; Get next patrol point from array
  (set `self.NextRotation` (`self.K2_GetActorLocation` (`|GetArrayItem` (`/Game/AI/AC_PatrolPath.PatrolPath` (`self.AC_PathNode`)) (`self.LocationIndex`))))
  ; Check if we're at last path point
  (if (>= (`self.RotationIndex`) (- (`KismetArrayLibrary.Array_Length` (`/Game/AI/AC_PatrolPath.PatrolPath` (`self.AC_PathNode`))) 1))
    ; If yes, reset index, otherwise bump
    (set `self.RotationIndex` 0)
    (else
      (`/Engine/EditorBlueprintResources/StandardMacros.IncrementInt` (`self.RotationIndex`)))))

(fn `UserConstructionScript`)