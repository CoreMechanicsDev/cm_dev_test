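; Enemy character Blueprint that chases a BP_NPC_Jeanne actor using AI movement.
; BeginPlay stores the first BP_NPC_Jeanne found in the level as its target.
; When PawnSensing sees any pawn, it moves to that stored target, and each successful move re-triggers the chase after a short delay.
; A DoOnce resets after each re-trigger but has nothing wired to its output.
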(event `self.ReceiveBeginPlay`
  ; Create array of targets
  (bind _outactors (`GameplayStatics.GetAllActorsOfClass` "/Game/Characters/BP_NPC_Jeanne.BP_NPC_Jeanne_C"))
  (set `self.MyTargets` (`|GetArrayItem` _outactors)))

(event `ChaseTarget`
  ; Chase target, show debug print once, move then reset do once
  (`|ExecutionSequence`
    (:`then_0`
      (`/Engine/EditorBlueprintResources/StandardMacros.DoOnce` false :!label _label))
    (:`then_1`
      (`|AIMoveTo` self (0.0 0.0 0.0) (`self.MyTargets`)
        (:`OnSuccess`
          (`KismetSystemLibrary.Delay` 3.0)
          (`self.ChaseTarget`)
          (goto _label :!via `Reset`))))))

(event `self.PawnSensing.OnSeePawn`
  (params (Pawn :type "Pawn Object Reference"))
  (`self.ChaseTarget`))

(fn `UserConstructionScript`)