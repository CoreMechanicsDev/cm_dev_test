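; BP_NPC_Jeanne is an NPC character that wanders at random and heads toward the player when it senses a pawn.
; From BeginPlay, RandomDestination moves it to a reachable point within a fixed radius of its current location, repeating after a short delay on success only.
; PawnSensing's OnSeePawn logs a detection and starts AIMoveTo on player character 0, without checking which pawn was seen.
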(event `RandomDestination`
  (`|AIMoveTo` self (`NavigationSystemV1.K2_GetRandomReachablePointInRadius` (`self.K2_GetActorLocation`) 500.0 null null) null
    (:`OnSuccess`
      (`KismetSystemLibrary.Delay` 1.0)
      (`self.RandomDestination`))))

(event `self.ReceiveBeginPlay`
  (`self.RandomDestination`))

(event `self.PawnSensing.OnSeePawn`
  (params (Pawn :type "Pawn Object Reference"))
  (`MyBlueprintFunctionLibrary.CM_LogPrint` "Player Detected")
  (`|AIMoveTo` self (0.0 0.0 0.0) (`GameplayStatics.GetPlayerCharacter` 0)))

(fn `UserConstructionScript`)