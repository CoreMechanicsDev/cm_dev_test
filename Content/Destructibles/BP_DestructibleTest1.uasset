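; Test Blueprint for a destructible actor built on a C++ Destructible class, reacting to changes in its health.
; The C++ health-change event logs old and new values, then calls ShakeMesh while health stays above zero.
; ShakeMesh only logs a message, and nothing handles zero health.
; Disconnected leftovers hold C++ function tests (random roll, mesh spin) and an unused delayed sound-and-destroy sequence, noted for moving to a Gameplay Effect or Cue.
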(event `self.OnHealthChanged`
  (params (OldValue :type "Float (single-precision)") (NewValue :type "Float (single-precision)"))
  ; This event was created in Destructible's C++ class and fires wenever health changes
  (`MyBlueprintFunctionLibrary.CM_LogPrint` (`KismetStringLibrary.Concat_StrStr` "Health Changed From " (`KismetStringLibrary.Conv_DoubleToString` OldValue) " to " (`KismetStringLibrary.Conv_DoubleToString` NewValue)))
  (if (> NewValue 0.0)
    (`self.ShakeMesh`)))

(event `ShakeMesh`
  ; This event was created in Destructible's C++ class and fires wenever health changes
  (`MyBlueprintFunctionLibrary.CM_LogPrint` "SHAKE"))

(event `self.TestEvent`
  ; Testing custom c++ events and functions
)

(event `self.ReceiveBeginPlay`
  ; Testing custom c++ events and functions
)

(fn `UserConstructionScript`)